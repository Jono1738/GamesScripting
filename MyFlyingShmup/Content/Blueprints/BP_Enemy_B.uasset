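; BP_Enemy_B is an enemy with two rail guns that fires bullet volleys automatically from BeginPlay onward.
; A looping timer calls ShootBullet, which plays a firing sound and spawns an enemy projectile at each of four spawn points.
; PlayAnimation switches both guns between idle and shoot animations by index, calling itself after a delay to return to idle.
; The file contains no targeting, movement or damage logic.
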(event `PlayAnimation`
  (params (Index :type Integer))
  (switch `int` Index
    (:`0`
      (`SkeletalMeshComponent.PlayAnimation` (`self.rail_gun1`) "/Game/Fab/Rail_Gun/Railidle.Railidle" true)
      (`SkeletalMeshComponent.PlayAnimation` (`self.rail_gun2`) "/Game/Fab/Rail_Gun/Railidle.Railidle" true))
    (:`1`
      (`SkeletalMeshComponent.PlayAnimation` (`self.rail_gun2`) "/Game/Fab/Rail_Gun/RailShoot.RailShoot" false)
      (`SkeletalMeshComponent.PlayAnimation` (`self.rail_gun1`) "/Game/Fab/Rail_Gun/RailShoot.RailShoot" false)
      (`KismetSystemLibrary.Delay` 2.0)
      (`self.PlayAnimation` 0))))

(event `self.ReceiveBeginPlay`
  (`self.PlayAnimation` 0)
  (`KismetSystemLibrary.K2_SetTimerDelegate` (delegate `ShootBullet`) 1.5 true true))

(event `ShootBullet`
  (`GameplayStatics.PlaySound2D` "/Game/Sound/Custom_Sounds/SFX_EnemyShootRandom.SFX_EnemyShootRandom" 1.0 1.0 0.0 null null)
  (`self.PlayAnimation` 1)
  (`|SpawnActorFromClass` "/Game/Blueprints/BP_Projectile_Enemy_bullet.BP_Projectile_Enemy_Bullet_C" (`SceneComponent.K2_GetComponentToWorld` (`self.BulletSpawnPoint1`)) "Undefined" "MultiplyWithRoot" null null)
  (`|SpawnActorFromClass` "/Game/Blueprints/BP_Projectile_Enemy_bullet.BP_Projectile_Enemy_Bullet_C" (`SceneComponent.K2_GetComponentToWorld` (`self.BulletSpawnPoint2`)) "Undefined" "MultiplyWithRoot" null null)
  (`|SpawnActorFromClass` "/Game/Blueprints/BP_Projectile_Enemy_bullet.BP_Projectile_Enemy_Bullet_C" (`SceneComponent.K2_GetComponentToWorld` (`self.BulletSpawnPoint3`)) "Undefined" "MultiplyWithRoot" null null)
  (`|SpawnActorFromClass` "/Game/Blueprints/BP_Projectile_Enemy_bullet.BP_Projectile_Enemy_Bullet_C" (`SceneComponent.K2_GetComponentToWorld` (`self.BulletSpawnPoint4`)) "Undefined" "MultiplyWithRoot" null null))

(fn `UserConstructionScript`)