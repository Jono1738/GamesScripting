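; Enemy spawner actor that keeps spawning random enemies from a class pool at random intervals, starting at BeginPlay.
; A timer spawns one enemy and re-queues itself with a new random delay.
; Each enemy appears at a random point on the start spline, rotated to face a random point on the end spline.
; All randomness draws from one random stream seeded with a fixed value.
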(event `self.ReceiveBeginPlay`
  (`KismetMathLibrary.SetRandomStreamSeed` (`self.RandomStream`))
  (`self.QueueEnemySpawn`))

(event `QueueEnemySpawn`
  (bind _returnvalue (`KismetSystemLibrary.K2_SetTimerDelegate` (delegate `SpawnEnemy`) (`KismetMathLibrary.RandomFloatInRangeFromStream` (`self.RandomStream`) 1.0 5.0) false true))
  (set `self.ReturnValue` _returnvalue))

(event `SpawnEnemy`
  (bind (_startlocation _endlocation) (`self.GetStartAndEndLocation`))
  (`|SpawnActorFromClass` (`KismetArrayLibrary.Array_RandomFromStream` (`self.EnemyClassPool`) (`self.RandomStream`)) (`KismetMathLibrary.MakeTransform` _startlocation (`KismetMathLibrary.FindLookAtRotation` _startlocation _endlocation)) "Undefined" "MultiplyWithRoot" null null)
  (`self.QueueEnemySpawn`))

(fn `GetStartAndEndLocation`
  (returns (StartLocation :type "Vector Structure") (EndLocation :type "Vector Structure"))
  (bind _returnvalue (`KismetMathLibrary.RandomFloatFromStream` (`self.RandomStream`)))
  (return (`SplineComponent.GetLocationAtTime` (`self.StartLocation`) _returnvalue "World" false) (`SplineComponent.GetLocationAtTime` (`self.EndLocation`) _returnvalue "World" false)))

(fn `UserConstructionScript`)