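; Destructible forcefield actor that absorbs damage until its life runs out.
; BeginPlay starts a non-spatialized 2D hum and keeps a reference to it.
; AnyDamage subtracts from the clamped Life value.
; At zero it stops the hum, plays a zap, spawns BP_ForcefieldExplosion at its location and destroys itself.
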(event `self.ReceiveBeginPlay`
  (bind _returnvalue (`GameplayStatics.SpawnSound2D` "/Game/Sound/Custom_Sounds/SFX_ForcefieldHum.SFX_ForcefieldHum" 1.0 1.0 0.0 null))
  (set `self.2DSound` _returnvalue))

(event `self.ReceiveAnyDamage`
  (params (Damage :type "Float (single-precision)") (DamageType :type "DamageType Object Reference") (InstigatedBy :type "Controller Object Reference") (DamageCauser :type "Actor Object Reference"))
  (bind _output_get (set `self.Life` (`KismetMathLibrary.FClamp` (- (`self.Life`) Damage) 0.0 150.0)))
  (if (== _output_get 0.0)
    (`AudioComponent.Stop` (`self.2DSound`))
    (`GameplayStatics.PlaySound2D` "/Game/Sound/Custom_Sounds/SFX_ForcefieldZap.SFX_ForcefieldZap" 1.0 1.0 0.0 null null)
    (`|SpawnActorFromClass` "/Game/Particles/BP_ForcefieldExplosion.BP_ForcefieldExplosion_C" (`KismetMathLibrary.MakeTransform` (`self.K2_GetActorLocation`)) "AlwaysSpawn" "MultiplyWithRoot" null null)
    (`self.K2_DestroyActor`)))

(fn `UserConstructionScript`)