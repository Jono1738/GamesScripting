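; Eagle enemy that homes in on the player pawn.
; Tick feeds the direction to the player into FloatingPawnMovement and turns the actor to face them in yaw only.
; A looping timer from BeginPlay cycles attack animations through nested FlipFlops, a fixed 1-3-2-3 order despite the "Random" event name, each returning to the run loop after a delay.
; BeginPlay also plays a delayed eagle sound; no damage logic is here.
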(event `self.ReceiveBeginPlay`
  (`parent.ReceiveBeginPlay`)
  (`self.PlayAnimation` 0)
  (`KismetSystemLibrary.K2_SetTimerDelegate` (delegate `RandomAttackAnimation`) 2.5 true true)
  (`KismetSystemLibrary.Delay` 3.0)
  (`GameplayStatics.PlaySound2D` "/Game/Sound/Custom_Sounds/SFX_Eagle.SFX_Eagle" 1.0 1.0 0.0 null null))

(event `RandomAttackAnimation`
  (`/Engine/EditorBlueprintResources/StandardMacros.FlipFlop`
    (:`A`
      (`/Engine/EditorBlueprintResources/StandardMacros.FlipFlop`
        (:`A`
          (`self.PlayAnimation` 1))
        (:`B`
          (`self.PlayAnimation` 2))))
    (:`B`
      (`self.PlayAnimation` 3))))

(event `self.ReceiveTick`
  (params (DeltaSeconds :type "Float (single-precision)"))
  (bind _returnvalue (`self.K2_GetActorLocation`))
  (bind _returnvalue_2 (`self.K2_GetActorLocation` (`GameplayStatics.GetPlayerPawn` 0)))
  (bind (_returnvalue_roll _returnvalue_pitch _returnvalue_yaw) (`KismetMathLibrary.BreakRotator` (`KismetMathLibrary.FindLookAtRotation` _returnvalue _returnvalue_2)))
  (`PawnMovementComponent.AddInputVector` (`self.FloatingPawnMovement`) (`KismetMathLibrary.GetDirectionUnitVector` _returnvalue _returnvalue_2) false)
  (`self.K2_SetActorRotation` (`KismetMathLibrary.MakeRotator` 0.0 0.0 _returnvalue_yaw)))

(event `PlayAnimation`
  (params (Index :type Integer))
  (bind _ma001_eagle (`self.ma001_Eagle`))
  (switch `int` Index
    (:`0`
      (`SkeletalMeshComponent.PlayAnimation` _ma001_eagle "/Game/Fab/ma001_Eagle/Animations/ma001_Run.ma001_Run" true))
    (:`1`
      (`SkeletalMeshComponent.PlayAnimation` _ma001_eagle "/Game/Fab/ma001_Eagle/Animations/ma001_Attack_01.ma001_Attack_01" false)
      (`KismetSystemLibrary.Delay` 1.0)
      (`self.PlayAnimation` 0))
    (:`2`
      (`SkeletalMeshComponent.PlayAnimation` _ma001_eagle "/Game/Fab/ma001_Eagle/Animations/ma001_Attack_02.ma001_Attack_02" false)
      (`KismetSystemLibrary.Delay` 1.0)
      (`self.PlayAnimation` 0))
    (:`3`
      (`SkeletalMeshComponent.PlayAnimation` _ma001_eagle "/Game/Fab/ma001_Eagle/Animations/ma001_Attack_03.ma001_Attack_03" false)
      (`KismetSystemLibrary.Delay` 1.0)
      (`self.PlayAnimation` 0))))

(fn `UserConstructionScript`
  (`parent.UserConstructionScript`))