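; BP_Base_Enemy is a base enemy that damages any actor overlapping it by an amount equal to its MaxHealth.
; Incoming damage lowers Health and updates a health bar in its widget component.
; Non-lethal hits play a sound and briefly flash static and skeletal meshes with an overlay material.
; Death plays a sound, triggers camera shake, adds MaxHealth to the player controller's score, spawns an explosion and destroys the enemy.
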(event `self.ReceiveActorBeginOverlap`
  (params (OtherActor :type "Actor Object Reference"))
  (`GameplayStatics.ApplyDamage` OtherActor (`self.MaxHealth`)))

(event `self.ReceiveAnyDamage`
  (params (Damage :type "Float (single-precision)") (DamageType :type "DamageType Object Reference") (InstigatedBy :type "Controller Object Reference") (DamageCauser :type "Actor Object Reference"))
  (`self.ApplyDamage` Damage)
  ; check if enemy health is 0, if so, start death seq
  (if (<= (`self.Health`) 0.0)
    (`GameplayStatics.PlaySound2D` "/Game/Sound/SFX_Essentials_FREE_SAMPLE/SFX_Essentials_16_BIRDS/Wavs/BIRDPrey_InsJ_Owl_Tawny-Male_Hooting_01-01_DRY.BIRDPrey_InsJ_Owl_Tawny-Male_Hooting_01-01_DRY" 1.0 1.0 0.0 null null)
    (`|ExecutionSequence`
      (:`then_0`
        (bind _asmy_player_controller (cast `/Game/Framework/myPlayerController` (`GameplayStatics.GetPlayerController` 0)))
        (`/Game/Framework/myPlayerController.ApplyCameraShake` _asmy_player_controller)
        (`/Game/Framework/myPlayerController.AddToScore` _asmy_player_controller (`self.MaxHealth`)))
      (:`then_1`
        (`|SpawnActorFromClass` "/Game/Particles/BP_Enemy_Death_Explosion.BP_Enemy_Death_Explosion_C" (`KismetMathLibrary.MakeTransform` (`self.K2_GetActorLocation`)) "AlwaysSpawn" "MultiplyWithRoot" null null))
      (:`then_2`
        (`self.K2_DestroyActor`)))
    (else
      (`GameplayStatics.PlaySound2D` "/Game/Sound/Custom_Sounds/SFX_EnemyOnHitRandom.SFX_EnemyOnHitRandom" 1.0 1.0 0.0 null null)
      (for _array_element (`self.K2_GetComponentsByClass` "/Script/Engine.StaticMeshComponent")
        (`MeshComponent.SetOverlayMaterial` _array_element "/Game/Materials/MI_Damage_Flash.MI_Damage_Flash"))
      (for _array_element_2 (`self.K2_GetComponentsByClass` "/Script/Engine.SkeletalMeshComponent")
        (`MeshComponent.SetOverlayMaterial` _array_element_2 "/Game/Materials/MI_Damage_Flash.MI_Damage_Flash"))
      (`KismetSystemLibrary.Delay` 0.2)
      (for _array_element_3 (`self.K2_GetComponentsByClass` "/Script/Engine.StaticMeshComponent")
        (`MeshComponent.SetOverlayMaterial` _array_element_3 null))
      (for _array_element_4 (`self.K2_GetComponentsByClass` "/Script/Engine.SkeletalMeshComponent")
        (`MeshComponent.SetOverlayMaterial` _array_element_4 null)))))

(event `self.ReceiveBeginPlay`
  (set `self.Health` (`self.MaxHealth`)))

(event `ApplyDamage`
  (params (Damage :type "Float (double-precision)"))
  (set `self.Health` (- (`self.Health`) Damage))
  ; Set progress bar of user widget within widget component
  (bind _aswbp_enemy_health_bar (cast `/Game/UI/WBP_Enemy_HealthBar` (`WidgetComponent.GetUserWidgetObject` (`self.Widget`))))
  (`/Game/UI/WBP_Enemy_HealthBar.SetHealth` _aswbp_enemy_health_bar (/ (`self.Health`) (`self.MaxHealth`))))

(event `self.Capsule.OnComponentHit`
  (params (HitComponent :type "PrimitiveComponent Object Reference") (OtherActor :type "Actor Object Reference") (OtherComp :type "PrimitiveComponent Object Reference") (NormalImpulse :type "Vector Structure") (Hit :type "HitResult Structure (by ref)")))

(event `self.Capsule.OnComponentBeginOverlap`
  (params (OverlappedComponent :type "PrimitiveComponent Object Reference") (OtherActor :type "Actor Object Reference") (OtherComp :type "PrimitiveComponent Object Reference") (OtherBodyIndex :type Integer) (bFromSweep :type Boolean) (SweepResult :type "HitResult Structure (by ref)")))

(event `self.Capsule.OnComponentEndOverlap`
  (params (OverlappedComponent :type "PrimitiveComponent Object Reference") (OtherActor :type "Actor Object Reference") (OtherComp :type "PrimitiveComponent Object Reference") (OtherBodyIndex :type Integer)))

(fn `UserConstructionScript`)