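; Enemy turret that yaws its base toward the player every tick and fires a volley of bullets from multiple spawn points on a looping timer.
; Non-lethal damage briefly flashes an overlay material on all static and skeletal meshes.
; At zero health it shakes the camera, adds MaxHealth to the score, spawns an explosion and optional pickup, then destroys itself.
; The pickup option and type are set through AssignSpawnedEnemyProps.
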(event `self.ReceiveTick`
  (params (DeltaSeconds :type "Float (single-precision)"))
  (bind (_returnvalue_roll _returnvalue_pitch _returnvalue_yaw) (`KismetMathLibrary.BreakRotator` (`KismetMathLibrary.FindLookAtRotation` (`self.K2_GetActorLocation`) (`self.K2_GetActorLocation` (`GameplayStatics.GetPlayerPawn` 0)))))
  (`SceneComponent.K2_SetWorldRotation` (`self.Base`) (`KismetMathLibrary.MakeRotator` 0.0 0.0 _returnvalue_yaw) false false))

(event `self.ReceiveAnyDamage`
  (params (Damage :type "Float (single-precision)") (DamageType :type "DamageType Object Reference") (InstigatedBy :type "Controller Object Reference") (DamageCauser :type "Actor Object Reference"))
  (`self.ApplyDamage` Damage)
  ; check if enemy health is 0, if so, start death seq
  (if (<= (`self.Health`) 0.0)
    (`GameplayStatics.PlaySound2D` "/Game/Sound/Custom_Sounds/SFX_Machine_Explode.SFX_Machine_Explode" 1.0 1.0 0.0 null null)
    (`|ExecutionSequence`
      (:`then_0`
        (bind _asmy_player_controller (cast `/Game/Framework/myPlayerController` (`GameplayStatics.GetPlayerController` 0)))
        (`/Game/Framework/myPlayerController.ApplyCameraShake` _asmy_player_controller)
        (`/Game/Framework/myPlayerController.AddToScore` _asmy_player_controller (`self.MaxHealth`)))
      (:`then_1`
        (`|SpawnActorFromClass` "/Game/Particles/BP_Explosion_2.BP_Explosion_2_C" (`KismetMathLibrary.MakeTransform` (`self.K2_GetActorLocation`)) "AlwaysSpawn" "MultiplyWithRoot" null null)
        (if (`self.Spawn Pick Up on Death`)
          (`|SpawnActorFromClass` (`self.Pick Up Type to Spawn`) (`KismetMathLibrary.Conv_VectorToTransform` (`self.K2_GetActorLocation`)) "AlwaysSpawn" "MultiplyWithRoot" null null)))
      (:`then_2`
        (`self.K2_DestroyActor`)))
    (else
      (`GameplayStatics.PlaySound2D` "/Game/Sound/Custom_Sounds/SFK_Machine_hit.SFK_Machine_hit" 1.0 1.0 0.0 null null)
      (for _array_element (`self.K2_GetComponentsByClass` "/Script/Engine.StaticMeshComponent")
        (`MeshComponent.SetOverlayMaterial` _array_element "/Game/Materials/MI_Damage_Flash.MI_Damage_Flash"))
      (for _array_element_2 (`self.K2_GetComponentsByClass` "/Script/Engine.SkeletalMeshComponent")
        (`MeshComponent.SetOverlayMaterial` _array_element_2 "/Game/Materials/MI_Damage_Flash.MI_Damage_Flash"))
      (`KismetSystemLibrary.Delay` 0.2)
      (for _array_element_3 (`self.K2_GetComponentsByClass` "/Script/Engine.StaticMeshComponent")
        (`MeshComponent.SetOverlayMaterial` _array_element_3 null))
      (for _array_element_4 (`self.K2_GetComponentsByClass` "/Script/Engine.SkeletalMeshComponent")
        (`MeshComponent.SetOverlayMaterial` _array_element_4 null)))))

(event `self.ReceiveBeginPlay`
  (`parent.ReceiveBeginPlay`)
  (`KismetSystemLibrary.K2_SetTimerDelegate` (delegate `ShootBullet`) 3.0 true true))

(event `ShootBullet`
  (bind (_returnvalue_location _returnvalue_rotation) (`KismetMathLibrary.BreakTransform` (`SceneComponent.K2_GetComponentToWorld` (`self.BulletSpawnL1`))))
  (bind (_returnvalue_location_2 _returnvalue_rotation_2) (`KismetMathLibrary.BreakTransform` (`SceneComponent.K2_GetComponentToWorld` (`self.BulletSpawnL2`))))
  (bind (_returnvalue_location_3 _returnvalue_rotation_3) (`KismetMathLibrary.BreakTransform` (`SceneComponent.K2_GetComponentToWorld` (`self.BulletSpawnR3`))))
  (bind (_returnvalue_location_4 _returnvalue_rotation_4) (`KismetMathLibrary.BreakTransform` (`SceneComponent.K2_GetComponentToWorld` (`self.BulletSpawnR4`))))
  (bind (_returnvalue_location_5 _returnvalue_rotation_5) (`KismetMathLibrary.BreakTransform` (`SceneComponent.K2_GetComponentToWorld` (`self.BulletSpawnL4`))))
  (bind (_returnvalue_location_6 _returnvalue_rotation_6) (`KismetMathLibrary.BreakTransform` (`SceneComponent.K2_GetComponentToWorld` (`self.BulletSpawnL3`))))
  (bind (_returnvalue_location_7 _returnvalue_rotation_7) (`KismetMathLibrary.BreakTransform` (`SceneComponent.K2_GetComponentToWorld` (`self.BulletSpawnR2`))))
  (bind (_returnvalue_location_8 _returnvalue_rotation_8) (`KismetMathLibrary.BreakTransform` (`SceneComponent.K2_GetComponentToWorld` (`self.BulletSpawnR1`))))
  (bind (_returnvalue_location_9 _returnvalue_rotation_9) (`KismetMathLibrary.BreakTransform` (`SceneComponent.K2_GetComponentToWorld` (`self.BulletSpawn1`))))
  (bind (_returnvalue_location_10 _returnvalue_rotation_10) (`KismetMathLibrary.BreakTransform` (`SceneComponent.K2_GetComponentToWorld` (`self.BulletSpawn2`))))
  (`GameplayStatics.PlaySound2D` "/Game/Sound/Custom_Sounds/SFX_EnemyShootRandom.SFX_EnemyShootRandom" 1.0 1.0 0.0 null null)
  (`|SpawnActorFromClass` "/Game/Blueprints/BP_Projectile_Enemy_bullet.BP_Projectile_Enemy_Bullet_C" (`KismetMathLibrary.MakeTransform` _returnvalue_location_9 _returnvalue_rotation_9) "AlwaysSpawn" "MultiplyWithRoot" null null)
  (`|SpawnActorFromClass` "/Game/Blueprints/BP_Projectile_Enemy_bullet.BP_Projectile_Enemy_Bullet_C" (`KismetMathLibrary.MakeTransform` _returnvalue_location_10 _returnvalue_rotation_10) "AlwaysSpawn" "MultiplyWithRoot" null null)
  (`|SpawnActorFromClass` "/Game/Blueprints/BP_Projectile_Enemy_bullet.BP_Projectile_Enemy_Bullet_C" (`KismetMathLibrary.MakeTransform` _returnvalue_location _returnvalue_rotation) "AlwaysSpawn" "MultiplyWithRoot" null null)
  (`|SpawnActorFromClass` "/Game/Blueprints/BP_Projectile_Enemy_bullet.BP_Projectile_Enemy_Bullet_C" (`KismetMathLibrary.MakeTransform` _returnvalue_location_2 _returnvalue_rotation_2) "AlwaysSpawn" "MultiplyWithRoot" null null)
  (`|SpawnActorFromClass` "/Game/Blueprints/BP_Projectile_Enemy_bullet.BP_Projectile_Enemy_Bullet_C" (`KismetMathLibrary.MakeTransform` _returnvalue_location_6 _returnvalue_rotation_6) "AlwaysSpawn" "MultiplyWithRoot" null null)
  (`|SpawnActorFromClass` "/Game/Blueprints/BP_Projectile_Enemy_bullet.BP_Projectile_Enemy_Bullet_C" (`KismetMathLibrary.MakeTransform` _returnvalue_location_5 _returnvalue_rotation_5) "AlwaysSpawn" "MultiplyWithRoot" null null)
  (`|SpawnActorFromClass` "/Game/Blueprints/BP_Projectile_Enemy_bullet.BP_Projectile_Enemy_Bullet_C" (`KismetMathLibrary.MakeTransform` _returnvalue_location_8 _returnvalue_rotation_8) "AlwaysSpawn" "MultiplyWithRoot" null null)
  (`|SpawnActorFromClass` "/Game/Blueprints/BP_Projectile_Enemy_bullet.BP_Projectile_Enemy_Bullet_C" (`KismetMathLibrary.MakeTransform` _returnvalue_location_7 _returnvalue_rotation_7) "AlwaysSpawn" "MultiplyWithRoot" null null)
  (`|SpawnActorFromClass` "/Game/Blueprints/BP_Projectile_Enemy_bullet.BP_Projectile_Enemy_Bullet_C" (`KismetMathLibrary.MakeTransform` _returnvalue_location_3 _returnvalue_rotation_3) "AlwaysSpawn" "MultiplyWithRoot" null null)
  (`|SpawnActorFromClass` "/Game/Blueprints/BP_Projectile_Enemy_bullet.BP_Projectile_Enemy_Bullet_C" (`KismetMathLibrary.MakeTransform` _returnvalue_location_4 _returnvalue_rotation_4) "AlwaysSpawn" "MultiplyWithRoot" null null))

(event `/Game/Framework/BPI_myFlyingShmup.AssignSpawnedEnemyProps`
  (params (SpawnPickUpOnDeath :type Boolean) (PickUpTypeToSpawn :type "/Game/Blueprints/BP_Base_PickUp Class Reference"))
  (set `self.Spawn Pick Up on Death` SpawnPickUpOnDeath)
  (set `self.Pick Up Type to Spawn` PickUpTypeToSpawn))

(fn `UserConstructionScript`
  (`parent.UserConstructionScript`))