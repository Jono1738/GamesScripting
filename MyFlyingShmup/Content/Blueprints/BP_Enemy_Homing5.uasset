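; Eagle enemy that flies along its own spline path, with a spawn sound on BeginPlay.
; The spline detaches in world space, then a timeline scaled by TravelTime moves the actor at constant velocity with sweep.
; Every timeline update re-issues the looping run animation through PlayAnimation.
; That event also offers three attack animations that revert to run after a delay, though nothing here triggers them, and no target homing appears.
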(event `self.ReceiveBeginPlay`
  (`parent.ReceiveBeginPlay`)
  (`GameplayStatics.PlaySound2D` "/Game/Sound/Custom_Sounds/SFX_EagleRunner.SFX_EagleRunner" 1.0 1.0 0.0 null null)
  (`SceneComponent.K2_DetachFromComponent` (`self.Spline`) "KeepWorld" "KeepWorld" "KeepWorld" true)
  (`TimelineComponent.SetPlayRate` (`self.MovingAlongSpline`) (/ 0.6 (`self.TravelTime`)))
  (bind (_direction _time) (`Timeline|MovingAlongSpline` :!via `PlayFromStart`)
    (:`Update`
      (`self.K2_SetActorLocation` (`SplineComponent.GetLocationAtTime` (`self.Spline`) _time "World" true) true)
      (`self.PlayAnimation` 0))))

(event `PlayAnimation`
  (params (Index :type Integer))
  (bind _ma001_eagle (`self.ma001_Eagle`))
  (switch `int` Index
    (:`0`
      (`SkeletalMeshComponent.PlayAnimation` _ma001_eagle "/Game/Fab/ma001_Eagle/Animations/ma001_Run.ma001_Run" true))
    (:`1`
      (`SkeletalMeshComponent.PlayAnimation` _ma001_eagle "/Game/Fab/ma001_Eagle/Animations/ma001_Attack_01.ma001_Attack_01" false)
      (`KismetSystemLibrary.Delay` 1.0)
      (`self.PlayAnimation` 0))
    (:`2`
      (`SkeletalMeshComponent.PlayAnimation` _ma001_eagle "/Game/Fab/ma001_Eagle/Animations/ma001_Attack_02.ma001_Attack_02" false)
      (`KismetSystemLibrary.Delay` 1.0)
      (`self.PlayAnimation` 0))
    (:`3`
      (`SkeletalMeshComponent.PlayAnimation` _ma001_eagle "/Game/Fab/ma001_Eagle/Animations/ma001_Attack_03.ma001_Attack_03" false)
      (`KismetSystemLibrary.Delay` 1.0)
      (`self.PlayAnimation` 0))))

(fn `UserConstructionScript`
  (`parent.UserConstructionScript`))